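; Game state for a platform match that runs the replicated pre-round countdown and signals the round's end.
; The authority decrements RoundCountDown each second, re-armed by its RepNotify, which also plays chimes and triggers the local controller's Ready-Go animation at 2.
; At zero it calls StartRound, which currently only casts the game mode.
; A WinnerRef change makes the authority set IsRoundEnded, whose RepNotify plays the whistle and match-over animation.
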(event `self.ReceiveBeginPlay`
  (`/Engine/EditorBlueprintResources/ActorMacros.Switch Has Authority`
    (:`Authority`
      (`self.CountDown`))))

(event `CountDown`
  (`KismetSystemLibrary.Delay` 1.0)
  (bind _result (`/Engine/EditorBlueprintResources/StandardMacros.DecrementInt` (`self.RoundCountDown`))
    (:`  `
      (set `self.RoundCountDown` _result))))

(fn `OnRep_IsRoundEnded`
  ; 경기종료
  (`GameplayStatics.PlaySound2D` "/Game/Audio/Cues/SC_RefereeWhistle.SC_RefereeWhistle" 1.0 1.0 0.0 null null)
  (bind _asbp_jms_platform_player_controller (cast `/Game/BP/Char/BP_JMS_PlatformPlayerController` (`GameplayStatics.GetPlayerController` 0)))
  (`/Game/BP/Char/BP_JMS_PlatformPlayerController.OwningClient_PlayMatchOverAnimation` _asbp_jms_platform_player_controller))

(fn `OnRep_RoundCountDown`
  (`self.PlayCountDownSound`)
  (`self.PlayReadyGoAnimmation`)
  (`/Engine/EditorBlueprintResources/ActorMacros.Switch Has Authority`
    (:`Authority`
      (if (== (`self.RoundCountDown`) 0)
        (`self.StartRound`)
        (else
          (`self.CountDown`))))))

(fn `OnRep_WinnerRef`
  (`/Engine/EditorBlueprintResources/ActorMacros.Switch Has Authority`
    (:`Authority`
      (set `self.IsRoundEnded` true) ; 경기 종료
    )))

(fn `PlayCountDownSound`
  (if (!= (`self.RoundCountDown`) 0)
    (`GameplayStatics.PlaySound2D` "/Game/Audio/Cues/SC_Countdown_chime.SC_Countdown_chime" 1.0 1.0 0.0 null null)
    (else
      (`GameplayStatics.PlaySound2D` "/Game/Audio/Cues/SC_Countdown_Chime_final.SC_Countdown_Chime_final" 1.0 1.0 0.0 null null))))

(fn `PlayReadyGoAnimmation`
  (if (== (`self.RoundCountDown`) 2)
    (bind _asbp_jms_platform_player_controller (cast `/Game/BP/Char/BP_JMS_PlatformPlayerController` (`GameplayStatics.GetPlayerController` 0)))
    (`/Game/BP/Char/BP_JMS_PlatformPlayerController.OwningClient_PlayReadyGoAnimation` _asbp_jms_platform_player_controller)))

(fn `StartRound`
  (cast `/Game/BP/Char/BP_JMS_PlatformGameMode` (`GameplayStatics.GetGameMode`)))

(fn `UserConstructionScript`)
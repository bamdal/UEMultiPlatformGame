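; Player controller for a multiplayer platform game that puts each player in as a character or spectator.
; On BeginPlay it retries GameState and PlayerState casts on a delay, caching GameMode on the server.
; The local controller then creates the HUD and, based on the round countdown, requests a spawn through GameMode.
; Character spawns await the PlayerState's color and use its checkpoint; match UI events and menu toggle are stubs.
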(event `self.ReceiveBeginPlay`
  ; 사용자 입력에 플레이어 입력과 플레이컨트롤러만 응답할 수 있는 모드로 설정
  (`WidgetBlueprintLibrary.SetInputMode_GameOnly` self)
  (`self.GetCasts`
    (:`NewParam2`
      (`self.InitPlayerController`))))

(event `SRSpawnCharacter`
  ; 플레이어캐릭터 스폰
  (bind _colorid (`self.GetAppearance`)
    (:`than`
      (set `self.IsPlayingPlayer` true)
      (`/Game/BP/Char/BP_JMS_PlatformGameMode.SpawnCharacter` (`self.As BP JMS Platform Game Mode`) self (`self.GetCurrentCheckPoint`) _colorid))))

(event `SR_SpawnSpectatingPawn`
  (params (SpawnAtPlayerLocaiton :type Boolean))
  ; 관전자 스폰
  (set `self.IsPlayingPlayer` false)
  (`/Game/BP/Char/BP_JMS_PlatformGameMode.SpawnSpectatePawn` (`self.As BP JMS Platform Game Mode`) self SpawnAtPlayerLocaiton (`KismetMathLibrary.MakeTransform` (0.0 0.0 0.0))))

(event `OwningClient_PlayReadyGoAnimation`
  (`KismetSystemLibrary.PrintString` "OC_PRGA"))

(event `OwningClient_PlayMatchOverAnimation`)

(fn `CreateGamePlayHUD`
  (bind _wbp_gameplayhud (`self.WBP_GamePlayHUD`)
    (:`then`
      (if (not (`Widget.IsInViewport` _wbp_gameplayhud))
        (`UserWidget.AddToViewport` (`self.WBP_GamePlayHUD`) 0)))
    (:`else`
      (bind _returnvalue (`|CreateWidget` "/Game/BP/UI/WBP_GamePlayHUD.WBP_GamePlayHUD_C" self))
      (bind _output_get (set `self.WBP_GamePlayHUD` _returnvalue))
      (`UserWidget.AddToViewport` _output_get 0))))

(fn `GetCurrentCheckPoint`
  (returns (`Check Point Tag` :type Name))
  (bind _as_bp_jms_platform_player_state (`self.As BP JMS Platform Player State`)
    (:`then`
      (return (`JMS_PlatformPlayerState.CheckPointTag` _as_bp_jms_platform_player_state)))
    (:`else`)))

(fn `InitPlayerController`
  (if (`self.IsLocalPlayerController`)
    ; HUD생성
    (`self.CreateGamePlayHUD`)
    ; Player, spectator결정
    (if (!= (`/Game/BP/Char/BP_JMS_PlatformGameState.RoundCountDown` (`self.As BP JMS Platform Game State`)) 0)
      (`self.SRSpawnCharacter`)
      (else
        (`self.SR_SpawnSpectatingPawn` false)))))

(fn `Toggle_WB_GameMenu`)

(fn `UserConstructionScript`)
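; Game mode for a multiplayer platformer that spawns and possesses player characters or spectator pawns and server-travels between two maps.
; Spawning claims an untagged PlayerStart by tagging it "Taken", or picks a random one matching the checkpoint tag.
; Characters receive an appearance color and stay frozen while the game state's round countdown is nonzero.
; EnableCharacterMovement restores walking and sphere-traces at each character, sending CollidedMessage to the hit actor.
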(fn `DestroyControlledPawn`
  (params (Player :type "Controller Object Reference"))
  (bind _returnvalue (`Controller.K2_GetPawn` Player))
  (`/Engine/EditorBlueprintResources/StandardMacros.IsValid` _returnvalue
    (:`Is Valid`
      (`self.K2_DestroyActor` _returnvalue))
    (:`Is Not Valid`
      _))
  (return))

(fn `EnableCharacterMovement`
  (for _array_element (`self.AllPlayerControllers`)
    (bind _returnvalue (`Controller.K2_GetPawn` _array_element))
    (bind _asbp_jms_platform_character (cast `/Game/BP/Char/BP_JMS_PlatformCharacter` _returnvalue))
    (`CharacterMovementComponent.SetMovementMode` (`Character.CharacterMovement` _asbp_jms_platform_character) "MOVE_Walking" 0)
    (bind _returnvalue_2 (`self.K2_GetActorLocation` _returnvalue))
    (bind _outhit (`KismetSystemLibrary.SphereTraceSingle` :`Start` _returnvalue_2 :`End` _returnvalue_2 :`Radius` 10.0 :`TraceChannel` "TraceTypeQuery1" :`DrawDebugType` "ForDuration" :`DrawTime` 2.0))
    (message `/Game/BP/Core/BPI_GamePlay.Collided` (`.HitActor` (`GameplayStatics.BreakHitResult` _outhit)) _asbp_jms_platform_character))
  (return))

(fn `GetAvailablePlayerStart`
  (returns (PlayerStartTransform :type "Transform Structure (by ref)"))
  ; PlayerStart에 tag가 비었다면 Taken입력후 return Transform
  (bind _outactors (`GameplayStatics.GetAllActorsOfClass` "/Script/Engine.PlayerStart"))
  (for _array_element _outactors
    (if (== (`PlayerStart.PlayerStartTag` _array_element) "None")
      (set `PlayerStart.PlayerStartTag` "Taken" _array_element)
      (break)))
  (return (`self.GetTransform` _array_element)))

(fn `GetCheckPointPlayerStart`
  (params (CheckPointId :type Name))
  (returns (CheckPointTransform :type "Transform Structure"))
  (locals (PlayerStarts :type "Array of PlayerStart Object Reference"))
  (bind _playerstarts (`local.PlayerStarts`))
  ; checkpointId와 같은 playerstart중 하나 선택
  (bind _outactors (`GameplayStatics.GetAllActorsOfClass` "/Script/Engine.PlayerStart"))
  (for _array_element _outactors
    (if (== (`PlayerStart.PlayerStartTag` _array_element) (`local.CheckPointId`))
      (`KismetArrayLibrary.Array_Add` (`local.PlayerStarts`) _array_element)))
  (`KismetArrayLibrary.Array_Shuffle` _playerstarts)
  (bind _output_get (set `local.PlayerStarts` _playerstarts))
  (return (`self.GetTransform` (`|GetArrayItem` _output_get))))

(fn `GetRandomPlayerStart`
  (returns (RandomPlayerStartTransform :type "Transform Structure (by ref)"))
  (bind _outactors (`GameplayStatics.GetAllActorsOfClass` "/Script/Engine.PlayerStart"))
  (return (`self.GetTransform` (`|GetArrayItem` _outactors (`KismetMathLibrary.RandomIntegerInRange` 0 (- (`KismetArrayLibrary.Array_Length` _outactors) 1))))))

(fn `SpawnCharacter`
  (params (Player :type "PlayerController Object Reference") (CheckPointTag :type Name) (AppearanceColorId :type Integer))
  (locals (SpawnTransform :type "Transform Structure"))
  (`self.DestroyControlledPawn` Player)
  (if (== CheckPointTag "None")
    (bind _playerstarttransform (`self.GetAvailablePlayerStart`))
    (set `local.SpawnTransform` _playerstarttransform)
    (else
      (bind _checkpointtransform (`self.GetCheckPointPlayerStart` (`local.CheckPointTag`)))
      (set `local.SpawnTransform` _checkpointtransform)))
  (bind _returnvalue (`|SpawnActorFromClass` "/Game/BP/Char/BP_JMS_PlatformCharacter.BP_JMS_PlatformCharacter_C" (`local.SpawnTransform`) "Undefined" "MultiplyWithRoot" (`local.Player`) null))
  (`Controller.Possess` (`local.Player`) _returnvalue)
  (`/Game/BP/Char/BP_JMS_PlatformCharacter.SR_SetAppearance` _returnvalue (`local.AppearanceColorId`))
  (bind _asbp_jms_platform_game_state (cast `/Game/BP/Char/BP_JMS_PlatformGameState` (`GameplayStatics.GetGameState`)))
  (if (not (== (`/Game/BP/Char/BP_JMS_PlatformGameState.RoundCountDown` _asbp_jms_platform_game_state) 0))
    (`CharacterMovementComponent.SetMovementMode` (`Character.CharacterMovement` _returnvalue) "MOVE_None" 0)))

(fn `SpawnSpectatePawn`
  (params (Player :type "Controller Object Reference") (SpawnAtPlayerLocaiton :type Boolean) (PlayerTransform :type "Transform Structure"))
  ; 관전자 생성
  (`self.DestroyControlledPawn` Player)
  (if SpawnAtPlayerLocaiton
    (bind _returnvalue (`|SpawnActorFromClass` "/Script/Engine.SpectatorPawn" (`local.PlayerTransform`) "Undefined" "MultiplyWithRoot" (`local.Player`) null))
    (`Controller.Possess` (`local.Player`) _returnvalue)
    (else
      (bind _returnvalue_2 (`|SpawnActorFromClass` "/Script/Engine.SpectatorPawn" (`self.GetRandomPlayerStart`) "Undefined" "MultiplyWithRoot" (`local.Player`) null))
      (`Controller.Possess` (`local.Player`) _returnvalue_2)))
  (return))

(fn `TravelToLevel`
  (bind _returnvalue (`GameplayStatics.GetCurrentLevelName` true))
  (switch `string` _returnvalue
    (:`L_NewMap1`
      ; 서버가 선택된 레벨로 접속한 Client전부를 데려간다
      (`KismetSystemLibrary.ExecuteConsoleCommand` (`KismetStringLibrary.Concat_StrStr` "ServerTravel/Game/Maps/" "L_NewMap2") null))
    (:`L_NewMap2`
      (`KismetSystemLibrary.ExecuteConsoleCommand` (`KismetStringLibrary.Concat_StrStr` "ServerTravel/Game/Maps/" "L_NewMap1") null))))

(fn `UserConstructionScript`)
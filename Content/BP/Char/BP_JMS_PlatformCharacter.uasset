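; BP_JMS_PlatformCharacter is a networked platformer character with spawn effects, color customization and respawning.
; On BeginPlay it plays a poof effect and sound through a server-to-multicast event chain.
; Collisions call a multicast ragdoll once via DoOnce, though the ragdoll, KillField and color OnRep bodies are empty.
; RespawnCharacter asks the owning BP_JMS_PlatformPlayerController to spawn a character on the server.
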(event `self.ReceiveBeginPlay`
  (`self.SR_SpawnPoof`))

(event `SR_SpawnPoof`
  (`self.MC_SpawnPoof`))

(event `MC_SpawnPoof`
  (bind _returnvalue (`self.K2_GetActorLocation`))
  (`NiagaraFunctionLibrary.SpawnSystemAtLocation` "/Game/Niagara/NS_Poof.NS_Poof" _returnvalue)
  (`GameplayStatics.PlaySoundAtLocation` "/Game/Audio/Cues/SC_Poof.SC_Poof" _returnvalue (struct) 1.0 1.0 0.0 "/Game/Audio/Classes/SA_Medium.SA_Medium" "/Game/Audio/Classes/SCC_Base.SCC_Base" null null))

(event `SR_SetAppearance`
  (params (AppearanceColorId :type Integer))
  ; 외형 꾸미기
  (set `self.Appearance Color Id` AppearanceColorId))

(event `/Game/BP/Core/BPI_GamePlay.Collided`
  (params (InteractingActor :type "Actor Object Reference"))
  (`/Engine/EditorBlueprintResources/StandardMacros.DoOnce` false
    (:`Completed`
      (`self.MC_Ragdoll`)
      (`KismetSystemLibrary.Delay` 0.2))))

(event `MC_Ragdoll`)

(event `/Game/BP/Core/BPI_GamePlay.KillField`)

(fn `OnRep_Appearance Color Id`)

(fn `RespawnCharacter`
  (bind _asbp_jms_platform_player_controller (cast `/Game/BP/Char/BP_JMS_PlatformPlayerController` (`PlayerState.GetPlayerController` (`GameplayStatics.GetPlayerState` 0))))
  ; 클라->서버 스폰요청
  (`/Game/BP/Char/BP_JMS_PlatformPlayerController.SRSpawnCharacter` _asbp_jms_platform_player_controller))

(fn `UserConstructionScript`)
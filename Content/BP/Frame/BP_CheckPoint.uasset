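; BP_CheckPoint is a checkpoint actor that records which checkpoint a platformer player last touched.
; On box overlap, only the authority writes its CheckPointId into the CheckPointTag of the character's BP_JMS_PlatformPlayerState.
; The construction script shows the ID on a TextRender label.
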(event `self.Box.OnComponentBeginOverlap`
  (params (OverlappedComponent :type "PrimitiveComponent Object Reference") (OtherActor :type "Actor Object Reference") (OtherComp :type "PrimitiveComponent Object Reference") (OtherBodyIndex :type Integer) (bFromSweep :type Boolean) (SweepResult :type "HitResult Structure (by ref)"))
  (`/Engine/EditorBlueprintResources/ActorMacros.Switch Has Authority`
    (:`Authority`
      (bind _asbp_jms_platform_character (cast `/Game/BP/Char/BP_JMS_PlatformCharacter` OtherActor))
      (bind _asbp_jms_platform_player_state (cast `/Game/BP/Char/BP_JMS_PlatformPlayerState` (`Pawn.PlayerState` _asbp_jms_platform_character)))
      (set `JMS_PlatformPlayerState.CheckPointTag` (`self.CheckPointId`) _asbp_jms_platform_player_state))))

(fn `UserConstructionScript`
  (`TextRenderComponent.K2_SetText` (`self.TextRender`) (`|FormatText` "CheckPoint : {a}" (`self.CheckPointId`))))
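; BP_Tropy is a trophy pickup that decides the winner of a networked platformer match.
; On mesh overlap, a server-only DoOnce casts the overlapping actor to the platform character and records its player state as the winner in the game state.
; MC_SpawnPoof, apparently a multicast by its prefix, then plays the poof effect and sound at the trophy, and the authority destroys the actor.
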(event `self.StaticMesh.OnComponentBeginOverlap`
  (params (OverlappedComponent :type "PrimitiveComponent Object Reference") (OtherActor :type "Actor Object Reference") (OtherComp :type "PrimitiveComponent Object Reference") (OtherBodyIndex :type Integer) (bFromSweep :type Boolean) (SweepResult :type "HitResult Structure (by ref)"))
  (`/Engine/EditorBlueprintResources/ActorMacros.Switch Has Authority`
    (:`Authority`
      (`/Engine/EditorBlueprintResources/StandardMacros.DoOnce` false
        (:`Completed`
          (bind _asbp_jms_platform_character (cast `/Game/BP/Char/BP_JMS_PlatformCharacter` OtherActor))
          (bind _asbp_jms_platform_game_state (cast `/Game/BP/Char/BP_JMS_PlatformGameState` (`GameplayStatics.GetGameState`)))
          (`JMS_PlatformGameState.SetWinnerRef` _asbp_jms_platform_game_state (`/Game/BP/Char/BP_JMS_PlatformCharacter.As BP JMS Platform Player State` _asbp_jms_platform_character))
          (`self.MC_SpawnPoof`))))))

(event `MC_SpawnPoof`
  (`NiagaraFunctionLibrary.SpawnSystemAtLocation` "/Game/Niagara/NS_Poof.NS_Poof" (`self.K2_GetActorLocation`))
  (`GameplayStatics.PlaySoundAtLocation` "/Game/Audio/Cues/SC_Poof.SC_Poof" (`self.K2_GetActorLocation`) (struct) 1.0 1.0 0.0 null null null null)
  (`/Engine/EditorBlueprintResources/ActorMacros.Switch Has Authority`
    (:`Authority`
      (`self.K2_DestroyActor`))))

(fn `UserConstructionScript`)
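; General Blueprint function library of UI helpers for showing popups, error messages and a loading screen.
; Popup and loading screen widgets are created for player controller 0 and added to the viewport only when that controller is local.
; Error helpers read network and travel error strings from BP_JMS_PlatformGI, showing one as a popup, network first, then clearing it.
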(fn `ClickFor_ActiveError`
  (bind _actove_error (`self.IsActiveError` null))
  (if _actove_error
    (bind _asbp_jms_platform_gi (cast `/Game/BP/Core/BP_JMS_PlatformGI` (`GameplayStatics.GetGameInstance` null)))
    (bind _jmsnetworkerror (`JMS_PlatformGI.JMSNetworkError` _asbp_jms_platform_gi))
    (if (`KismetStringLibrary.IsEmpty` _jmsnetworkerror)
      (bind _jmstravelerror (`JMS_PlatformGI.JMSTravelError` _asbp_jms_platform_gi))
      (if (not (`KismetStringLibrary.IsEmpty` _jmstravelerror))
        (`self.CreateErrorPopup` _jmstravelerror)
        (set `JMS_PlatformGI.JMSTravelError` "" _asbp_jms_platform_gi))
      (else
        (`self.CreateErrorPopup` _jmsnetworkerror)
        (set `JMS_PlatformGI.JMSNetworkError` "" _asbp_jms_platform_gi)))
    (return)))

(fn `Create_LodingScreen`
  (bind _returnvalue (`GameplayStatics.GetPlayerController` null))
  (if (`Controller.IsLocalPlayerController` _returnvalue)
    (bind _returnvalue_2 (`|CreateWidget` "/Game/BP/UI/WBP_LodingScreen.WBP_LodingScreen_C" _returnvalue))
    (`UserWidget.AddToViewport` _returnvalue_2 0)))

(fn `CreateErrorPopup`
  (params (B :type String))
  (`self.CreatePopup` (`|GenericToText` (`KismetStringLibrary.Concat_StrStr` "Error" B)) "OK"))

(fn `CreatePopup`
  (params (PopupMessage :type Text) (ConfirmButtonText :type Text) (DeclineButtonText :type Text) (ShowRightButton :type Boolean))
  (returns (OutputPin :type "/Game/BP/UI/WBP_Popup Object Reference"))
  (bind _returnvalue (`GameplayStatics.GetPlayerController` null))
  (if (`Controller.IsLocalPlayerController` _returnvalue)
    (bind _returnvalue_2 (`|CreateWidget` "/Game/BP/UI/WBP_Popup.WBP_Popup_C" _returnvalue PopupMessage ConfirmButtonText DeclineButtonText ShowRightButton))
    (`UserWidget.AddToViewport` _returnvalue_2 0)
    (return _returnvalue_2)))

(fn `IsActiveError`
  (returns (`Actove Error` :type Boolean))
  (bind _asbp_jms_platform_gi (cast `/Game/BP/Core/BP_JMS_PlatformGI` (`GameplayStatics.GetGameInstance` null)))
  (if (`KismetStringLibrary.IsEmpty` (`JMS_PlatformGI.JMSNetworkError` _asbp_jms_platform_gi))
    (if (`KismetStringLibrary.IsEmpty` (`JMS_PlatformGI.JMSTravelError` _asbp_jms_platform_gi))
      (return false)
      (else
        (return true)))
    (else
      (return true))))